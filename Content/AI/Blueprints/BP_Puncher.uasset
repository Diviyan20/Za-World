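; BP_Puncher is an enemy AI character that reacts to player punches and to boom, electric, ice and stun effects.
; Punches reward the player a charge, then share a health-decrement path with boom and electric hits, ending in kill count, poof effect and destruction.
; Knuckle stun pauses movement through timed montages, while ice only swaps the material temporarily.
; GetIdealRange supplies attack and defend radii, and SetMovementSpeed returns zero.
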(event Custom|DamagedOutline
  (Rendering|Material|SetOverlayMaterial (Variables|Character|GetMesh) "/Game/Materials/Masters/MM_Outline.MM_Outline" :!class /Script/Engine.MeshComponent)
  (Utilities|FlowControl|Delay 0.1)
  (Rendering|Material|SetOverlayMaterial (Variables|Character|GetMesh) 0 :!class /Script/Engine.MeshComponent))

(event EventBoomDamage
  (Niagara|SpawnSystematLocation "/Game/VFX/Niagara_System/NS_Boom.NS_Boom" (Transformation|GetWorldLocation (Variables|Character|GetMesh)) "0, 0, 0" "1.500000,1.500000,1.500000")
  ;[1 1 1] Get Damaged by Player
  (CallFunction|DamagedOutline)
  (bind _output_get (Variables|Default|SetHealth (- (Variables|Default|GetHealth) 1.0)))
  (if (== _output_get 0.0)
    (Audio|PlaySound2D "/Game/SFX/Enemy_Dies.Enemy_Dies" 1.0 1.0 0.0 0 0)
    (Math|Integer|IncrementInt (Variables|/Game/FirstPerson/Blueprints/BP_MC.BP_MC_C|GetKillCount (Variables|Default|GetChar%20REF))
      (:%20%20
        (Components|Activation|Activate (Variables|Default|GetPoof) false)
        (Rendering|SetVisibility (Variables|Character|GetMesh) false false)
        (Utilities|FlowControl|Delay 0.8)
        (Actor|DestroyActor)))))

(event EventIceSlow
  (bind _mesh (Variables|Character|GetMesh))
  (Rendering|Material|SetMaterial _mesh 0 "/Game/Materials/MM_LBlue.MM_LBlue")
  (Utilities|FlowControl|Delay 2e+01)
  (Rendering|Material|SetMaterial _mesh 0 "/Game/AI/Characters/Meshes/Y-Bot/M_Ranged.M_Ranged"))

(event EventBeginPlay
  (Utilities|FlowControl|Sequence
    (:then_0
      (Components|Activation|Deactivate (Variables|Default|GetPoof)))
    (:then_1
      (Components|Activation|Deactivate (Variables|Default|GetStunned)))))

(event EventKnuckleStun
  ;[1 1 1] Stun Animation
  (Pawn|Components|CharacterMovement|DisableMovement (Variables|Character|GetCharacterMovement))
  (Animation|PlayAnimMontage "/Game/AI/Characters/Animations/Y-Bot/Puncher/AM_Stunned.AM_Stunned" 1.0 "None")
  (Components|Activation|Activate (Variables|Default|GetStunned) false)
  (Utilities|FlowControl|Delay 5.0)
  (Components|Activation|Deactivate (Variables|Default|GetStunned))
  (Animation|PlayAnimMontage "/Game/AI/Characters/Animations/Y-Bot/Puncher/AM_GettingUp.AM_GettingUp" 1.0 "None")
  (Utilities|FlowControl|Delay 4.0)
  (Pawn|Components|CharacterMovement|SetMovementMode (Variables|Character|GetCharacterMovement) "MOVE_Walking" 0))

(event EventElectricDamage
  ;[1 1 1] Get Damaged by Player
  (bind _output_get (Variables|Default|SetHealth (- (Variables|Default|GetHealth) 1.0)))
  (if (== _output_get 0.0)
    (Audio|PlaySound2D "/Game/SFX/Enemy_Dies.Enemy_Dies" 1.0 1.0 0.0 0 0)
    (Math|Integer|IncrementInt (Variables|/Game/FirstPerson/Blueprints/BP_MC.BP_MC_C|GetKillCount (Variables|Default|GetChar%20REF))
      (:%20%20
        (Components|Activation|Activate (Variables|Default|GetPoof) false)
        (Rendering|SetVisibility (Variables|Character|GetMesh) false false)
        (Utilities|FlowControl|Delay 0.8)
        (Actor|DestroyActor)))))

(event EventEnemyDamage
  ;[1 1 1] Get Damaged by Player
  (if (not (Variables|Default|GetisDead?))
    (bind _asbp_mc (Utilities|Casting|CastToBP_MC (Game|GetPlayerCharacter 0)))
    (Variables|Default|SetChar%20REF _asbp_mc)
    (Variables|/Game/FirstPerson/Blueprints/BP_MC.BP_MC_C|SetPunchCharges (Variables|Default|GetChar%20REF) (+ (Variables|/Game/FirstPerson/Blueprints/BP_MC.BP_MC_C|GetPunchCharges (Variables|Default|GetChar%20REF)) 1))
    (Default|EnablePowFX (Variables|Default|GetChar%20REF))
    (Audio|PlaySound2D "/Game/SFX/Punching.Punching" 1.0 1.0 0.0 0 0)
    (Audio|PlaySound2D "/Game/SFX/Enemy_Hit.Enemy_Hit" 1.0 1.0 0.0 0 0)
    (CallFunction|DamagedOutline)
    (bind _output_get (Variables|Default|SetHealth (- (Variables|Default|GetHealth) 1.0)))
    (if (== _output_get 0.0)
      (Audio|PlaySound2D "/Game/SFX/Enemy_Dies.Enemy_Dies" 1.0 1.0 0.0 0 0)
      (Math|Integer|IncrementInt (Variables|/Game/FirstPerson/Blueprints/BP_MC.BP_MC_C|GetKillCount (Variables|Default|GetChar%20REF))
        (:%20%20
          (Components|Activation|Activate (Variables|Default|GetPoof) false)
          (Rendering|SetVisibility (Variables|Character|GetMesh) false false)
          (Utilities|FlowControl|Delay 0.8)
          (Actor|DestroyActor))))))

(fn ConstructionScript
  (|CallParentFunction))

(fn GetIdealRange
  (return 0.0 1.3e+02))

(fn SetMovementSpeed
  (params (Speed :type E_MovementSpeed%20Enum :default "NewEnumerator0"))
  (return 0.0))