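; BP_ParangMan is a machete-wielding melee AI enemy that slashes the player and reports ideal attack and defend ranges.
; SlashMachete plays a montage, applies damage through a box overlap on its notify, then signals attack end.
; Punch and boom hits share one damage path with a white overlay flash, health loss and death; punches also grant the player charges.
; IceSlow only swaps the material temporarily, without changing speed.
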(event Custom|Slash%20Machete
  ;[1 1 1] - Play Slash Animation
  ; - Deal Damage to Player
  (Animation|Montage|PlayMontage (Variables|Character|GetMesh) "/Game/AI/Characters/Animations/Y-Bot/ParangMan/AM_Slash.AM_Slash"
    (:OnCompleted
      (Default|CallOnAttackEnd :!label _label))
    (:OnInterrupted
      (goto _label))
    (:OnNotifyBegin
      (bind _outactors (Collision|BoxOverlapActors (Transformation|GetWorldLocation (Variables|Default|GetBox)) "5.000000,5.000000,5.000000" (Utilities|Array|MakeArray "ObjectTypeQuery3") "/Game/FirstPerson/Blueprints/BP_MC.BP_MC_C" (Utilities|Array|MakeArray self) :!class /Script/Engine.KismetSystemLibrary))
      (for _array_element _outactors
        (Game|Damage|ApplyDamage _array_element 4e+01 (Pawn|GetController) self)))))

(event Custom|DamagedOutline
  (Rendering|Material|SetOverlayMaterial (Variables|Character|GetMesh) "/Game/Materials/MM_White.MM_White" :!class /Script/Engine.MeshComponent)
  (Utilities|FlowControl|Delay 0.2)
  (Rendering|Material|SetOverlayMaterial (Variables|Character|GetMesh) 0 :!class /Script/Engine.MeshComponent))

(event EventIceSlow
  (bind _mesh (Variables|Character|GetMesh))
  (Rendering|Material|SetMaterial _mesh 0 "/Game/Materials/MM_LBlue.MM_LBlue")
  (Utilities|FlowControl|Delay 2e+01)
  (Rendering|Material|SetMaterial _mesh 0 "/Game/AI/Characters/Meshes/Y-Bot/M_Melee.M_Melee"))

(event EventBoomDamage
  ;[1 1 1] Get Damaged by the Player
  (CallFunction|DamagedOutline)
  (bind _output_get (Variables|Default|SetHealth (- (Variables|Default|GetHealth) 1.0)))
  (if (== _output_get 0.0)
    (Audio|PlaySound2D "/Game/SFX/Enemy_Dies.Enemy_Dies" 1.0 1.0 0.0 0 0)
    (Math|Integer|IncrementInt (Variables|/Game/FirstPerson/Blueprints/BP_MC.BP_MC_C|GetKillCount (Variables|Default|GetChar%20REF))
      (:%20%20
        (Pawn|Components|CharacterMovement|DisableMovement (Variables|Character|GetCharacterMovement))
        (Variables|Default|SetisDead? true)
        (Animation|PlayAnimMontage "/Game/AI/Characters/Animations/Y-Bot/Puncher/AM_PuncherDeath.AM_PuncherDeath" 1.0 "None")
        (Utilities|FlowControl|Delay 1.0)
        (Actor|DestroyActor)))))

(event EventEnemyDamage
  ;[1 1 1] Get Damaged by the Player
  (if (not (Variables|Default|GetisDead?))
    (bind _asbp_mc (Utilities|Casting|CastToBP_MC (Game|GetPlayerCharacter 0)))
    (Variables|Default|SetChar%20REF _asbp_mc)
    (Variables|/Game/FirstPerson/Blueprints/BP_MC.BP_MC_C|SetPunchCharges (Variables|Default|GetChar%20REF) (+ (Variables|/Game/FirstPerson/Blueprints/BP_MC.BP_MC_C|GetPunchCharges (Variables|Default|GetChar%20REF)) 1))
    (Default|EnablePowFX (Variables|Default|GetChar%20REF))
    (Audio|PlaySound2D "/Game/SFX/Punching.Punching" 1.0 1.0 0.0 0 0)
    (Audio|PlaySound2D "/Game/SFX/Enemy_Hit.Enemy_Hit" 1.0 1.0 0.0 0 0)
    (CallFunction|DamagedOutline)
    (bind _output_get (Variables|Default|SetHealth (- (Variables|Default|GetHealth) 1.0)))
    (if (== _output_get 0.0)
      (Audio|PlaySound2D "/Game/SFX/Enemy_Dies.Enemy_Dies" 1.0 1.0 0.0 0 0)
      (Math|Integer|IncrementInt (Variables|/Game/FirstPerson/Blueprints/BP_MC.BP_MC_C|GetKillCount (Variables|Default|GetChar%20REF))
        (:%20%20
          (Pawn|Components|CharacterMovement|DisableMovement (Variables|Character|GetCharacterMovement))
          (Variables|Default|SetisDead? true)
          (Animation|PlayAnimMontage "/Game/AI/Characters/Animations/Y-Bot/Puncher/AM_PuncherDeath.AM_PuncherDeath" 1.0 "None")
          (Utilities|FlowControl|Delay 1.0)
          (Actor|DestroyActor))))))

(fn ConstructionScript
  (|CallParentFunction))

(fn GetIdealRange
  (return 1e+02 1.3e+02))

(fn SetMovementSpeed
  (params (Speed :type E_MovementSpeed%20Enum :default "NewEnumerator0"))
  (return 0.0))