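; FatMan enemy character that punches the player and reacts to hits, ice and knuckle stuns.
; Punch deals damage through a sphere overlap on the montage notify, then signals attack end.
; EnemyDamage grants the player punch charges and joins BoomDamage's health countdown, which at zero counts the kill, plays death effects and destroys the actor.
; Stun temporarily disables movement; IceSlow only swaps the material, and SetMovementSpeed is a stub returning zero.
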(event Custom|Punch
  ;[1 1 1] - Play Punch Animation
  ; - Deal Damage to Player
  (Animation|Montage|PlayMontage (Variables|Character|GetMesh) "/Game/AI/Characters/Animations/FatMan/AM_FatmanPunch.AM_FatmanPunch" 1.5
    (:OnCompleted
      (Default|CallOnAttackEnd :!label _label))
    (:OnInterrupted
      (goto _label))
    (:OnNotifyBegin
      (bind _outactors (Collision|SphereOverlapActors (Transformation|GetWorldLocation (Variables|Default|GetSphere)) 25.0 (Utilities|Array|MakeArray "ObjectTypeQuery3") 0 (Utilities|Array|MakeArray self)))
      (for _array_element _outactors
        (Game|Damage|ApplyDamage _array_element 2e+01 (Pawn|GetController) self)))))

(event Custom|DamagedOutline
  (Rendering|Material|SetOverlayMaterial (Variables|Character|GetMesh) "/Game/Materials/Masters/MM_Outline.MM_Outline" :!class /Script/Engine.MeshComponent)
  (Utilities|FlowControl|Delay 0.2)
  (Rendering|Material|SetOverlayMaterial (Variables|Character|GetMesh) 0 :!class /Script/Engine.MeshComponent))

(event Custom|Destroy%20Actor
  ;[1 1 1] Damage
  (Actor|DestroyActor))

(event EventBeginPlay
  (Utilities|FlowControl|Sequence
    (:then_0
      (Components|Activation|Deactivate (Variables|Default|GetPoof)))
    (:then_1
      (Components|Activation|Deactivate (Variables|Default|GetStunned)))))

(event EventIceSlow
  (bind _mesh (Variables|Character|GetMesh))
  (Rendering|Material|SetMaterial _mesh 0 "/Game/Materials/MM_LBlue.MM_LBlue")
  (Utilities|FlowControl|Delay 2e+01)
  (Rendering|Material|SetMaterial _mesh 0 "/Game/AI/Characters/Meshes/FatMan/Ch43_Body.Ch43_Body"))

(event EventEnemyDamage
  ;[1 1 1] Damage
  (if (not (Variables|Default|GetisDead?))
    (bind _asbp_mc (Utilities|Casting|CastToBP_MC (Game|GetPlayerCharacter 0)))
    (bind _output_get (Variables|Default|SetAs%20BP%20MC _asbp_mc))
    (Variables|/Game/FirstPerson/Blueprints/BP_MC.BP_MC_C|SetPunchCharges _output_get (+ (Variables|/Game/FirstPerson/Blueprints/BP_MC.BP_MC_C|GetPunchCharges (Variables|Default|GetAs%20BP%20MC)) 1))
    (Default|EnablePowFX (Variables|Default|GetAs%20BP%20MC))
    (Audio|PlaySound2D "/Game/SFX/Punching.Punching" 1.0 1.0 0.0 0 0)
    (Audio|PlaySound2D "/Game/SFX/Enemy_Hit.Enemy_Hit" 1.0 1.0 0.0 0 0)
    (CallFunction|DamagedOutline)
    (bind _output_get_2 (Variables|Default|SetHealth (- (Variables|Default|GetHealth) 1.0)))
    (if (== _output_get_2 0.0)
      (Audio|PlaySound2D "/Game/SFX/Enemy_Dies.Enemy_Dies" 1.0 1.0 0.0 0 0)
      (Math|Integer|IncrementInt (Variables|/Game/FirstPerson/Blueprints/BP_MC.BP_MC_C|GetKillCount (Variables|Default|GetAs%20BP%20MC))
        (:%20%20
          (Pawn|Components|CharacterMovement|DisableMovement (Variables|Character|GetCharacterMovement))
          (Variables|Default|SetisDead? true)
          (bind _returnvalue (Animation|PlayAnimMontage "/Game/AI/Characters/Animations/Y-Bot/Puncher/AM_PuncherDeath.AM_PuncherDeath" 1.0 "None"))
          (Utilities|FlowControl|Delay _returnvalue)
          (Components|Activation|Activate (Variables|Default|GetPoof) false)
          (Utilities|Time|SetTimerbyEvent (delegate Custom|Destroy%20Actor) 0.25))))))

(event EventBoomDamage
  ;[1 1 1] Damage
  (bind _output_get (Variables|Default|SetHealth (- (Variables|Default|GetHealth) 1.0)))
  (if (== _output_get 0.0)
    (Audio|PlaySound2D "/Game/SFX/Enemy_Dies.Enemy_Dies" 1.0 1.0 0.0 0 0)
    (Math|Integer|IncrementInt (Variables|/Game/FirstPerson/Blueprints/BP_MC.BP_MC_C|GetKillCount (Variables|Default|GetAs%20BP%20MC))
      (:%20%20
        (Pawn|Components|CharacterMovement|DisableMovement (Variables|Character|GetCharacterMovement))
        (Variables|Default|SetisDead? true)
        (bind _returnvalue (Animation|PlayAnimMontage "/Game/AI/Characters/Animations/Y-Bot/Puncher/AM_PuncherDeath.AM_PuncherDeath" 1.0 "None"))
        (Utilities|FlowControl|Delay _returnvalue)
        (Components|Activation|Activate (Variables|Default|GetPoof) false)
        (Utilities|Time|SetTimerbyEvent (delegate Custom|Destroy%20Actor) 0.25)))))

(event EventKnuckleStun
  ;[1 1 1] Stun Anmation
  (Pawn|Components|CharacterMovement|DisableMovement (Variables|Character|GetCharacterMovement))
  (Animation|PlayAnimMontage "/Game/AI/Characters/Animations/FatMan/AM_Stunned.AM_Stunned" 1.0 "None")
  (Components|Activation|Activate (Variables|Default|GetStunned) false)
  (Utilities|FlowControl|Delay 5.0)
  (Components|Activation|Deactivate (Variables|Default|GetStunned))
  (Animation|PlayAnimMontage "/Game/AI/Characters/Animations/FatMan/AM_GettingUp.AM_GettingUp" 1.0 "None")
  (Utilities|FlowControl|Delay 4.0)
  (Pawn|Components|CharacterMovement|SetMovementMode (Variables|Character|GetCharacterMovement) "MOVE_Walking" 0))

(fn ConstructionScript
  (|CallParentFunction))

(fn GetIdealRange
  (return 0.0 1.3e+02))

(fn SetMovementSpeed
  (params (Speed :type E_MovementSpeed%20Enum :default "NewEnumerator0"))
  (return 0.0))