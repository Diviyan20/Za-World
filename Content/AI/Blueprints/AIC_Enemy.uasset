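; AI controller for enemies that sends its pawn after the player as soon as it is possessed.
; On possess, it waits briefly, runs the BT_Enemy_Melee behavior tree, then calls SetStateAsAttacking with the first player's character.
; That function writes the AttackTarget object and State enum blackboard keys, with no perception or other condition checked first.
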(event EventPossess
  (params (PossessedPawn :type Pawn%20Object%20Reference))
  (Utilities|FlowControl|Delay 0.2)
  (AI|RunBehaviorTree "/Game/AI/Behavior_Tree/BT_Enemy_Melee.BT_Enemy_Melee")
  (CallFunction|SetStateasAttacking (Game|GetPlayerCharacter 0)))

(fn ConstructionScript)

(fn SetStateasAttacking
  (params (AttackTarget :type Actor%20Object%20Reference))
  (bind _blackboard (Variables|Default|GetBlackboard))
  (AI|Components|Blackboard|SetValueasObject _blackboard (Variables|Keys|GetAttackTarget) AttackTarget)
  (AI|Components|Blackboard|SetValueasEnum _blackboard (Variables|Keys|GetState) (Utilities|Enum|LiteralenumE_States "NewEnumerator1")))